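; Tank pawn Blueprint that serves both player input and AI-controlled tanks.
; BeginPlay wires barrel, turret and tracks into the TankAiming and TankMovement components, links the health bar widget, and sets AI materials when possessed by a TankAIController.
; Input drives track throttles directly or movement intents through TankMovement, rotates the azimuth gimbal and spring arm for camera aim, and fires through TankAiming.
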(event EventBeginPlay
  (bind _returnvalue (Pawn|GetController))
  (Class|TankAimingComponent|Initialize (Variables|Default|GetTankAiming) (Variables|Default|GetBarrel) (Variables|Default|GetTurret))
  (Class|TankMovementComponent|Initialize (Variables|Default|GetTankMovement) (Variables|Default|GetLeft%20Track) (Variables|Default|GetRight%20Track))
  (CallFunction|InitializeHealthBarWidget)
  (bind _astank_aicontroller (Utilities|Casting|CastToTankAIController _returnvalue))
  (Class|TankAIController|SetAIMaterial _astank_aicontroller (Pawn|GetControlledPawn _returnvalue) "/Game/Tank/AI_Tank_High_MAT.AI_Tank_High_MAT" "/Game/Tank/AI_Tank_Low_MAT.AI_Tank_Low_MAT" (Variables|Default|GetTank) (Variables|Default|GetTurret) (Variables|Default|GetBarrel) (Variables|Default|GetLeft%20Track) (Variables|Default|GetRight%20Track)))

(event Input|ActionEvents|InputActionFire
  (params (Key :type Key%20Structure))
  ;[1 1 1] Camera Input Binding
  (:Pressed
    (Class|TankAimingComponent|Fire (Variables|Default|GetTankAiming) (Pawn|GetControlledPawn (Pawn|GetController)))))

(event Input|AxisEvents|InputAxisAimAzimuth
  (params (AxisValue :type Float%20%28single-precision%29))
  ;[1 1 1] Camera Input Binding
  (Transformation|AddLocalRotation (Variables|Default|GetAzimuth%20Gimbal) (Math|Rotator|MakeRotator 0.0 0.0 AxisValue) false false))

(event Input|AxisEvents|InputAxisMoveBackward
  (params (AxisValue :type Float%20%28single-precision%29))
  ;[1 1 1] Movement Input Binding
  (Class|TankMovementComponent|IntendMoveForward (Variables|Default|GetTankMovement) (+ (stale Input|AxisEvents|InputAxisMoveForward AxisValue) AxisValue)))

(event Input|AxisEvents|InputAxisTurnRight
  (params (AxisValue :type Float%20%28single-precision%29))
  ;[1 1 1] Movement Input Binding
  (Class|TankMovementComponent|IntendTurnRight (Variables|Default|GetTankMovement) AxisValue))

(event Input|AxisEvents|InputAxisAimElevation
  (params (AxisValue :type Float%20%28single-precision%29))
  ;[1 1 1] Camera Input Binding
  (Transformation|AddLocalRotation (Variables|Default|GetSpringArm) (Math|Rotator|MakeRotator 0.0 AxisValue 0.0) false false))

(event Input|AxisEvents|InputAxisLeftTrackThrottle
  (params (AxisValue :type Float%20%28single-precision%29))
  ;[1 1 1] Movement Input Binding
  (Class|TankTrack|SetThrottle (Variables|Default|GetLeft%20Track) AxisValue))

(event Input|AxisEvents|InputAxisRightTrackThrottle
  (params (AxisValue :type Float%20%28single-precision%29))
  ;[1 1 1] Movement Input Binding
  (Class|TankTrack|SetThrottle (Variables|Default|GetRight%20Track) AxisValue))

(event Input|AxisEvents|InputAxisTurnLeft
  (params (AxisValue :type Float%20%28single-precision%29))
  ;[1 1 1] Movement Input Binding
  (Class|TankMovementComponent|IntendTurnLeft (Variables|Default|GetTankMovement) AxisValue))

(event Input|AxisEvents|InputAxisMoveForward
  (params (AxisValue :type Float%20%28single-precision%29))
  ;[1 1 1] Movement Input Binding
  (Class|TankMovementComponent|IntendMoveForward (Variables|Default|GetTankMovement) (+ AxisValue (stale Input|AxisEvents|InputAxisMoveBackward AxisValue))))

(fn ConstructionScript)

(fn InitializeHealthBarWidget
  (bind _ashealth_bar (Utilities|Casting|CastToHealthBar (UserInterface|GetUserWidgetObject (Variables|Default|GetWidget))))
  (Variables|/Game/Blueprints/HealthBar.HealthBar_C|SetMyTank _ashealth_bar self)
  (return))